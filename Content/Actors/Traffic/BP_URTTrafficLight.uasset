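; Traffic light actor that displays vehicle red, yellow and green signals plus pedestrian signals and a countdown.
; BeginPlay and BPLightChanged call SetUpLights, which sets light intensities for the current state.
; Yellow also checks the previous state, keeping red lit when coming from red.
; Red shows the countdown text from RedTime and starts a looping one-second timer that decrements it, with no explicit clear here.
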(event EventBeginPlay
  (CallFunction|SetUpLights))

(event Collision|EventActorBeginOverlap
  (params (OtherActor :type Actor%20Object%20Reference)))

(event EventTick
  (params (DeltaSeconds :type Float%20%28single-precision%29)))

(event EventBPLightChanged
  (CallFunction|SetUpLights))

(fn ConstructionScript)

(fn SetUpLights
  (switch Utilities|FlowControl|Switch|SwitchonELightState (Variables|Default|GetCurrentLightState)
    (:Green
      (CallFunction|SetGreenLights))
    (:Yellow
      (CallFunction|SetYellowLights))
    (:Red
      (CallFunction|SetRedLights))))

(fn SetYellowLights
  (Rendering|SetVisibility (Variables|Default|GetCountdown) false false)
  (Rendering|Components|Light|SetIntensity (Variables|Default|GetGreen_Pedestrian) 0.0)
  (Rendering|Components|Light|SetIntensity (Variables|Default|GetYellow_Up) 9e+03)
  (switch Utilities|FlowControl|Switch|SwitchonELightState (Variables|Default|GetPreviousLightState)
    (:Green
      (Rendering|Components|Light|SetIntensity (Variables|Default|GetRed_Up) 0.0))
    (:Red
      (Rendering|Components|Light|SetIntensity (Variables|Default|GetRed_Up) 9e+03)
      (Rendering|Components|Light|SetIntensity (Variables|Default|GetGreen_Up) 0.0))))

(fn SetGreenLights
  (Rendering|Components|Light|SetIntensity (Variables|Default|GetGreen_Up) 9e+03)
  (Rendering|Components|Light|SetIntensity (Variables|Default|GetRed_Up) 0.0)
  (Rendering|SetVisibility (Variables|Default|GetCountdown) false false))

(fn SetRedLights
  (bind _countdown (Variables|Default|GetCountdown))
  (Rendering|Components|Light|SetIntensity (Variables|Default|GetRed_Up) 9e+03)
  (Rendering|Components|Light|SetIntensity (Variables|Default|GetYellow_Down) 0.0)
  (Rendering|Components|TextRender|SetText _countdown (Utilities|Text|ToText(Float) (Variables|Default|GetRedTime) "HalfToEven"))
  (Rendering|SetVisibility _countdown true false)
  (CallFunction|CreateCountdownTimer))

(fn CreateCountdownTimer
  (bind _returnvalue (Utilities|Time|SetTimerbyFunctionName self "UpdatePedestrianCountdown" 1.0 true 0.08))
  (Variables|Default|SetCountdownTimer _returnvalue))

(fn UpdatePedestrianCountdown
  (if (Utilities|Time|IsValidTimerHandle (Variables|Default|GetCountdownTimer))
    (bind _result (Math|Integer|DecrementInt (Math|Conversions|ToInteger(Byte) (Utilities|String|ToString(Text) (Variables|/Script/Engine.TextRenderComponent|GetText (Variables|Default|GetCountdown)))))
      (:%20%20
        (Rendering|Components|TextRender|SetText (Variables|Default|GetCountdown) (Utilities|Text|ToText(Integer) _result))))))